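; AI character that runs a scripted coin-collecting route across platforms, using lists from the game mode's coin counter.
; SetCoinToCollect advances a non-looping MultiGate through six fixed stages, chaining AIMoveTo calls to platforms and the first listed coin with hand-timed delays.
; Completed stages re-trigger the event until the last, and some platform moves retry on failure.
; JumptoDestination, not called here, launches the character in an arc toward a point above its destination.
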(event `self.ReceiveBeginPlay`
  (bind _asbp_third_person_game_mode (cast `/Game/ThirdPerson/Blueprints/BP_ThirdPersonGameMode` (`GameplayStatics.GetGameMode`)))
  (set `self.GM_Ref` _asbp_third_person_game_mode)
  (`self.Set coin to collect`))

(event `/Game/Platform/AI/BPI_Platform_AI_Character.JumpToDestination`
  (params (Destination :type "Vector Structure"))
  (bind _outlaunchvelocity (`GameplayStatics.SuggestProjectileVelocity_CustomArc` (`self.K2_GetActorLocation`) (`KismetMathLibrary.MakeVector` (.x Destination) (.y Destination) (+ (.z Destination) 300.0))))
  (`self.LaunchCharacter` _outlaunchvelocity true true))

(event `Set coin to collect`
  (bind _coin_counter_ref (`/Game/ThirdPerson/Blueprints/BP_ThirdPersonGameMode.Coin_Counter_Ref` (`self.GM_Ref`)))
  (bind _platform_list (`/Game/Platform/Blueprint/BP_Coin_Counter.Platform_List` _coin_counter_ref))
  (bind _returnvalue (`self.K2_GetActorLocation` (`|GetArrayItem` _platform_list 2)))
  (bind _returnvalue_2 (`self.K2_GetActorLocation` (`|GetArrayItem` (`/Game/Platform/Blueprint/BP_Coin_Counter.AI_Coin_List` _coin_counter_ref))))
  (`|MultiGate` false
    (:`Out 0`
      (`|AIMoveTo` self _returnvalue_2 null 20.0
        (:`OnSuccess`
          (`self.Set Coin To Collect`))))
    (:`Out 1`
      (`|AIMoveTo` self (`self.K2_GetActorLocation` (`|GetArrayItem` _platform_list)) null 50.0
        (:`OnSuccess`
          (`KismetSystemLibrary.Delay` 2.75)
          (`|AIMoveTo` self _returnvalue_2 null 20.0
            (:`OnSuccess`
              (`self.Set Coin To Collect`))))))
    (:`Out 2`
      (`|AIMoveTo` self (`self.K2_GetActorLocation` (`|GetArrayItem` _platform_list 1)) null 20.0
        (:`OnSuccess`
          (`KismetSystemLibrary.Delay` 2.75)
          (`|AIMoveTo` self _returnvalue_2 null 20.0
            (:`OnSuccess`
              (`self.Set Coin To Collect`))))))
    (:`Out 3`
      (`|AIMoveTo` self _returnvalue null 20.0
        (:`OnSuccess`
          (`KismetSystemLibrary.Delay` 1.75)
          (`|AIMoveTo` self _returnvalue_2 null 20.0
            (:`OnSuccess`
              (`KismetSystemLibrary.Delay` 1.8)
              (`|AIMoveTo` self _returnvalue null 20.0 :!label _label
                (:`OnSuccess`
                  (`KismetSystemLibrary.Delay` 1.1)
                  (`self.Set Coin To Collect`))
                (:`OnFail`
                  (`KismetSystemLibrary.Delay` 0.2)
                  (goto _label))))))))
    (:`Out 4`
      (`|AIMoveTo` self (`self.K2_GetActorLocation` (`|GetArrayItem` _platform_list 3)) null 20.0 :!label _label_2
        (:`OnSuccess`
          (`KismetSystemLibrary.Delay` 2.75)
          (`|AIMoveTo` self _returnvalue_2 null 20.0
            (:`OnSuccess`
              (`self.Set Coin To Collect`))))
        (:`OnFail`
          (`KismetSystemLibrary.Delay` 0.2)
          (goto _label_2))))
    (:`Out 5`
      (`|AIMoveTo` self _returnvalue_2 null 20.0))))

(fn `UserConstructionScript`)