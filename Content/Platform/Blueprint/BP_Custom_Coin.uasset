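; BP_Custom_Coin is a collectible coin for the platform minigame that adds to the score when overlapped.
; BeginPlay caches the game instance and the third-person game mode, though only the game mode is used afterwards.
; Any overlap on its Box adds SilverCoinScore to the game mode's PlatformMiniGameScore, calls AllCoinCollected with itself, then destroys the coin, without filtering the overlapping actor.
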(event `self.ReceiveBeginPlay`
  (bind _asbp_game_instance (cast `/Game/Blueprints/BP_GameInstance` (`GameplayStatics.GetGameInstance`)))
  (set `self.GI_Ref` _asbp_game_instance)
  ;[0 1 0] CPP :
  ; UPROPERTY(BlueprintReadWrite, EditDefaultOnly, Category="Default")
  ; TObjectPtr<ABP_ThirdPersonGameMode_C> GM_Ref;
  (bind _asbp_third_person_game_mode (cast `/Game/ThirdPerson/Blueprints/BP_ThirdPersonGameMode` (`GameplayStatics.GetGameMode`)))
  (set `self.GM_Ref` _asbp_third_person_game_mode))

(event `self.Box.OnComponentBeginOverlap`
  (params (OverlappedComponent :type "PrimitiveComponent Object Reference") (OtherActor :type "Actor Object Reference") (OtherComp :type "PrimitiveComponent Object Reference") (OtherBodyIndex :type Integer) (bFromSweep :type Boolean) (SweepResult :type "HitResult Structure (by ref)"))
  (bind _gm_ref (`self.GM_Ref`))
  ;[0 1 0] CPP :
  ; Void ACustomCoin::OnBoxBeginOverlap(UPrimitiveComponent* OverlappedComp, AActor* OtherActor, UPrimitiveComponent* OtherComp, int32 OtherBodyIndex, bool bFromSweep, const FHitResult& SweepResult)
  ; {
  ;      GM_Ref->PlatformMiniGameScore = GI_Ref->PlatformMiniGameScore + SiverCoinScore
  ; }
  (set `/Game/ThirdPerson/Blueprints/BP_ThirdPersonGameMode.Platform_MiniGame_Score` (+ (`/Game/ThirdPerson/Blueprints/BP_ThirdPersonGameMode.Platform_MiniGame_Score` _gm_ref) (`self.Silver_Coin_Score`)) _gm_ref)
  (`/Game/ThirdPerson/Blueprints/BP_ThirdPersonGameMode.All Coin Collected ?` (`self.GM_Ref`) self)
  (`self.K2_DestroyActor`))

(fn `UserConstructionScript`)