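; Golden coin pickup for the platform AI minigame, built as a child Blueprint that calls its parent's BeginPlay and construction script.
; Any overlap on its Box reports the coin to GMRef via AllAICoinCollected, adds GoldenCoinScore to PlatformAIMiniGameScore, then destroys the coin.
; The overlap handler does not check which actor triggered it.
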(event `self.ReceiveBeginPlay`
  (`parent.ReceiveBeginPlay`))

(event `self.Box.OnComponentBeginOverlap`
  (params (OverlappedComponent :type "PrimitiveComponent Object Reference") (OtherActor :type "Actor Object Reference") (OtherComp :type "PrimitiveComponent Object Reference") (OtherBodyIndex :type Integer) (bFromSweep :type Boolean) (SweepResult :type "HitResult Structure (by ref)"))
  (bind _gm_ref (`self.GM_Ref`))
  (`/Game/ThirdPerson/Blueprints/BP_ThirdPersonGameMode.All AI Coin Collected ?` (`self.GM_Ref`) self)
  (set `/Game/ThirdPerson/Blueprints/BP_ThirdPersonGameMode.Platform_AI_MiniGame_Score` (+ (`/Game/ThirdPerson/Blueprints/BP_ThirdPersonGameMode.Platform_AI_MiniGame_Score` _gm_ref) (`self.Golden_Coin_Score`)) _gm_ref)
  (`self.K2_DestroyActor`))

(fn `UserConstructionScript`
  (`parent.UserConstructionScript`))