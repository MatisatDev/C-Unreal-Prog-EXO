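; A gold coin pickup for the platform minigame that awards score when collected.
; On any overlap with its Box component, it adds its gold coin score to the platform minigame score held through GMRef.
; It then passes itself to AllCoinCollected on that reference and destroys itself.
; BeginPlay and the construction script only call the parent class.
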(event `self.ReceiveBeginPlay`
  (`parent.ReceiveBeginPlay`))

(event `self.Box.OnComponentBeginOverlap`
  (params (OverlappedComponent :type "PrimitiveComponent Object Reference") (OtherActor :type "Actor Object Reference") (OtherComp :type "PrimitiveComponent Object Reference") (OtherBodyIndex :type Integer) (bFromSweep :type Boolean) (SweepResult :type "HitResult Structure (by ref)"))
  (bind _gm_ref (`self.GM_Ref`))
  (set `/Game/ThirdPerson/Blueprints/BP_ThirdPersonGameMode.Platform_MiniGame_Score` (+ (`/Game/ThirdPerson/Blueprints/BP_ThirdPersonGameMode.Platform_MiniGame_Score` _gm_ref) (`self.Gold_Coin_Score`)) _gm_ref)
  (`/Game/ThirdPerson/Blueprints/BP_ThirdPersonGameMode.All Coin Collected ?` (`self.GM_Ref`) self)
  (`self.K2_DestroyActor`))

(fn `UserConstructionScript`
  (`parent.UserConstructionScript`))