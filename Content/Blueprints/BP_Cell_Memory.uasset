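; BP_Cell_Memory is a board cell that launches the Memory minigame.
; Its Action stores the given player ID in the game instance as the minigame player, then opens the Memory map.
; It also returns a per-player world position from two socket components, using SocketP0 for player 0 and SocketP1 for any other ID.
; BeginPlay and construction only defer to the parent class.
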(event `self.ReceiveBeginPlay`
  (`parent.ReceiveBeginPlay`))

(fn `Action`
  (params (PlayerId :type Integer))
  (set `/Game/Blueprints/BP_GameInstance.Mini Game Player Id` PlayerId (`self.As BP Game Instance`))
  (`GameplayStatics.OpenLevelBySoftObjectPtr` "/Game/Maps/MemoryMap.MemoryMap"))

(fn `GetSocketPosByPlayerId`
  (params (PlayerId :type Integer))
  (returns (SocketPosition :type "Vector Structure"))
  (locals (`Temp Socket Pos` :type "Vector Structure"))
  (if (== PlayerId 0)
    (set `local.Temp Socket Pos` (`SceneComponent.K2_GetComponentLocation` (`self.SocketP0`)))
    (else
      (set `local.Temp Socket Pos` (`SceneComponent.K2_GetComponentLocation` (`self.SocketP1`)))))
  (return (`local.Temp Socket Pos`)))

(fn `UserConstructionScript`
  (`parent.UserConstructionScript`))