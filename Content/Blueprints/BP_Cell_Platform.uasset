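; BP_Cell_Platform is a cell that launches the platform minigame for a player, extending a parent class.
; GetSocketPosByPlayerId returns the world location of one of four socket components, using a MultiGate with the player ID as start index in place of a switch.
; Action stores the player ID in the game instance as MiniGamePlayerId, then opens PlatformMap.
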(event `self.ReceiveBeginPlay`
  (`parent.ReceiveBeginPlay`))

(fn `Action`
  (params (PlayerId :type Integer))
  (set `/Game/Blueprints/BP_GameInstance.Mini Game Player Id` PlayerId (`self.As BP Game Instance`))
  (`GameplayStatics.OpenLevelBySoftObjectPtr` "/Game/Maps/PlatformMap.PlatformMap"))

(fn `GetSocketPosByPlayerId`
  (params (PlayerId :type Integer))
  (returns (SocketPosition :type "Vector Structure"))
  (locals (TempSocketPose :type "Vector Structure"))
  (`|MultiGate` false false PlayerId
    (:`Out 0`
      (set `local.TempSocketPose` (`SceneComponent.K2_GetComponentLocation` (`self.SocketP0`))))
    (:`Out 1`
      (set `local.TempSocketPose` (`SceneComponent.K2_GetComponentLocation` (`self.SocketP1`))))
    (:`Out 2`
      (set `local.TempSocketPose` (`SceneComponent.K2_GetComponentLocation` (`self.SocketP2`))))
    (:`Out 3`
      (set `local.TempSocketPose` (`SceneComponent.K2_GetComponentLocation` (`self.SocketP3`)))))
  (return (`local.TempSocketPose`)))

(fn `UserConstructionScript`
  (`parent.UserConstructionScript`))