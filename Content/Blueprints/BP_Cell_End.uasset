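; Final board cell for a game of up to four players that awards score to the landing player and detects the end of the match.
; Action counts each player on cell 17 once, flagging them as finished in the game instance.
; When that count equals PlayerTurnValue, it shows WB_END with the highest scorer's one-based number as winner.
; GetSocketPosByPlayerId uses a MultiGate to return each player's socket location.
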(fn `Action`
  (params (PlayerId :type Integer))
  (locals (`Score To Add` :type Integer :default 30) (`Player Scores` :type "Array of Integer"))
  (bind _finished_player (`self.Finished Player`))
  (bind _player_scores (`local.Player Scores`))
  (bind _player_turn_value (`/Game/Blueprints/BP_GameInstance.Player Turn Value` (`self.As BP Game Instance`)))
  (bind _number_of_finished_player (`/Game/Blueprints/BP_GameInstance.Number of Finished player` (`self.As BP Game Instance`)))
  (bind _playerlist (`/Game/Blueprints/BP_GameInstance.PlayerList` (`self.As BP Game Instance`)))
  (`/Game/Blueprints/BP_GameInstance.SetPlayerScoreByPlayerId` (`self.As BP Game Instance`) PlayerId (`local.Score To Add`))
  (`|ExecutionSequence`
    (:`then_0`
      (bind _playercellnumber (`/Game/Blueprints/BP_GameInstance.GetPlayerCellNumberByPlayerId` (`self.As BP Game Instance`) 0))
      (if (== _playercellnumber 17)
        (`/Engine/EditorBlueprintResources/StandardMacros.DoOnce` (`|GetArrayItem` (`/Game/Blueprints/BP_GameInstance.Number of Finished player` (`self.As BP Game Instance`)))
          (:`Completed`
            (`/Engine/EditorBlueprintResources/StandardMacros.IncrementInt` (`self.Finished Player`)
              (:`  `
                (`KismetArrayLibrary.Array_Set` _number_of_finished_player 0 true)))))))
    (:`then_1`
      (bind _playercellnumber_2 (`/Game/Blueprints/BP_GameInstance.GetPlayerCellNumberByPlayerId` (`self.As BP Game Instance`) 1))
      (if (== _playercellnumber_2 17)
        (`/Engine/EditorBlueprintResources/StandardMacros.DoOnce` (`|GetArrayItem` (`/Game/Blueprints/BP_GameInstance.Number of Finished player` (`self.As BP Game Instance`)) 1)
          (:`Completed`
            (`/Engine/EditorBlueprintResources/StandardMacros.IncrementInt` (`self.Finished Player`)
              (:`  `
                (`KismetArrayLibrary.Array_Set` _number_of_finished_player 1 true)))))))
    (:`then_2`
      (bind _playercellnumber_3 (`/Game/Blueprints/BP_GameInstance.GetPlayerCellNumberByPlayerId` (`self.As BP Game Instance`) 2))
      (if (== _playercellnumber_3 17)
        (`/Engine/EditorBlueprintResources/StandardMacros.DoOnce` (`|GetArrayItem` (`/Game/Blueprints/BP_GameInstance.Number of Finished player` (`self.As BP Game Instance`)) 2)
          (:`Completed`
            (`/Engine/EditorBlueprintResources/StandardMacros.IncrementInt` (`self.Finished Player`)
              (:`  `
                (`KismetArrayLibrary.Array_Set` _number_of_finished_player 2 true)))))))
    (:`then_3`
      (bind _playercellnumber_4 (`/Game/Blueprints/BP_GameInstance.GetPlayerCellNumberByPlayerId` (`self.As BP Game Instance`) 3))
      (if (== _playercellnumber_4 17)
        (`/Engine/EditorBlueprintResources/StandardMacros.DoOnce` (`|GetArrayItem` (`/Game/Blueprints/BP_GameInstance.Number of Finished player` (`self.As BP Game Instance`)) 3)
          (:`Completed`
            (`/Engine/EditorBlueprintResources/StandardMacros.IncrementInt` (`self.Finished Player`)
              (:`  `
                (`KismetArrayLibrary.Array_Set` _number_of_finished_player 3 true)))))))
    (:`then_4`
      (`KismetSystemLibrary.PrintString` (`KismetStringLibrary.Conv_IntToString` _player_turn_value))
      (`KismetSystemLibrary.PrintString` (`KismetStringLibrary.Conv_IntToString` _finished_player))
      (if (== _finished_player _player_turn_value)
        (bind _returnvalue (`|CreateWidget` "/Game/Widget/WB_END.WB_END_C"))
        (bind _output_get (set `self.WB_End_Ref` _returnvalue))
        (`UserWidget.AddToViewport` _output_get 0)
        (`KismetArrayLibrary.Array_Add` _player_scores (`.Score_4_09C81F4044D8FFB79AE82DA3832970A2` (break `/Game/Blueprints/S_PlayerData` (`|GetArrayItem` _playerlist))))
        (`KismetArrayLibrary.Array_Add` _player_scores (`.Score_4_09C81F4044D8FFB79AE82DA3832970A2` (break `/Game/Blueprints/S_PlayerData` (`|GetArrayItem` _playerlist 1))))
        (`KismetArrayLibrary.Array_Add` _player_scores (`.Score_4_09C81F4044D8FFB79AE82DA3832970A2` (break `/Game/Blueprints/S_PlayerData` (`|GetArrayItem` _playerlist 2))))
        (`KismetArrayLibrary.Array_Add` _player_scores (`.Score_4_09C81F4044D8FFB79AE82DA3832970A2` (break `/Game/Blueprints/S_PlayerData` (`|GetArrayItem` _playerlist 3))))
        (bind _result (`/Engine/EditorBlueprintResources/StandardMacros.IncrementInt` (`KismetMathLibrary.MaxOfIntArray` _player_scores))
          (:`  `
            (set `TextBlock.Text` (`KismetTextLibrary.Conv_IntToText` _result) (`/Game/Widget/WB_END.TextBlock_Winner` (`self.WB_End_Ref`)))))))))

(fn `GetSocketPosByPlayerId`
  (params (PlayerId :type Integer))
  (returns (SocketPosition :type "Vector Structure"))
  (locals (TempSocketPose :type "Vector Structure"))
  (`|MultiGate` false false PlayerId
    (:`Out 0`
      (set `local.TempSocketPose` (`SceneComponent.K2_GetComponentLocation` (`self.SocketP0`))))
    (:`Out 1`
      (set `local.TempSocketPose` (`SceneComponent.K2_GetComponentLocation` (`self.SocketP1`))))
    (:`Out 2`
      (set `local.TempSocketPose` (`SceneComponent.K2_GetComponentLocation` (`self.SocketP2`))))
    (:`Out 3`
      (set `local.TempSocketPose` (`SceneComponent.K2_GetComponentLocation` (`self.SocketP3`)))))
  (return (`local.TempSocketPose`)))

(fn `UserConstructionScript`
  (`parent.UserConstructionScript`))