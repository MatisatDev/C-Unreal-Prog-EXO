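; BP_Cell_Avance is a board cell that moves a player's pawn by a set number of extra cells when its action runs.
; Action reads the player's current cell number from the game instance, adds NbrDeCasesEnPlus, and has the game mode move the pawn there.
; GetSocketPosByPlayerId returns the world location of SocketP0 for player 0 and SocketP1 for any other ID.
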(event `self.ReceiveBeginPlay`
  (`parent.ReceiveBeginPlay`))

(fn `Action`
  (params (PlayerId :type Integer))
  (locals (`Nbr de cases en plus` :type Integer :default 1))
  (bind _playercellnumber (`/Game/Blueprints/BP_GameInstance.GetPlayerCellNumberByPlayerId` (`self.As BP Game Instance`) PlayerId))
  (`/Game/Blueprints/BP_GameMode.MovePawn` (`self.As BP Game Mode`) (+ _playercellnumber (`local.Nbr de cases en plus`)) PlayerId))

(fn `GetSocketPosByPlayerId`
  (params (PlayerId :type Integer))
  (returns (SocketPosition :type "Vector Structure"))
  (locals (`Temp Socket Pos` :type "Vector Structure"))
  (if (== PlayerId 0)
    (set `local.Temp Socket Pos` (`SceneComponent.K2_GetComponentLocation` (`self.SocketP0`)))
    (else
      (set `local.Temp Socket Pos` (`SceneComponent.K2_GetComponentLocation` (`self.SocketP1`)))))
  (return (`local.Temp Socket Pos`)))

(fn `UserConstructionScript`
  (`parent.UserConstructionScript`))