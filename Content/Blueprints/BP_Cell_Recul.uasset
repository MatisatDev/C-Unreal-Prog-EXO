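; BP_Cell_Recul is a board cell that sends a player's pawn backward when its Action runs.
; Action gets the player's current cell number from the game instance, subtracts NdrDeCasesEnMoins, and asks the game mode to move the pawn there.
; The subtraction has no bounds check in this Blueprint, and the event graph and construction script add no logic of their own.
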(fn `Action`
  (params (PlayerId :type Integer))
  (locals (`Ndr de cases en moins` :type Integer :default 1))
  (bind _playercellnumber (`/Game/Blueprints/BP_GameInstance.GetPlayerCellNumberByPlayerId` (`self.As BP Game Instance`) PlayerId))
  (`/Game/Blueprints/BP_GameMode.MovePawn` (`self.As BP Game Mode`) (- _playercellnumber (`local.Ndr de cases en moins`)) PlayerId))

(fn `UserConstructionScript`
  (`parent.UserConstructionScript`))