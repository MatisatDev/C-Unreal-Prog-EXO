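; Game mode for a card-matching memory minigame that hands results back to the players in BP_GameInstance.
; OnCardClicked holds the first card, then compares colors on the second, destroying a match for points or turning both cards back.
; After every comparison, unconditionally, whichever of the first two players sits on cell 3 gains MemoryScore, a variable separate from the running Score, and Test_map opens.
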(event `self.ReceiveBeginPlay`
  (bind _asbp_game_instance (cast `/Game/Blueprints/BP_GameInstance` (`GameplayStatics.GetGameInstance`)))
  (set `self.GI_Ref` _asbp_game_instance))

(fn `OnCardClicked`
  (params (Card :type "/Game/Memory/Blueprint/BP_Card Object Reference"))
  (bind _playerlist (`/Game/Blueprints/BP_GameInstance.PlayerList` (`self.GI_Ref`)))
  (bind _playerlist_2 (`/Game/Blueprints/BP_GameInstance.PlayerList` (`self.GI_Ref`)))
  (bind (_playerid _score _cellnumber) (break `/Game/Blueprints/S_PlayerData` (`|GetArrayItem` _playerlist_2 1)))
  (bind (_playerid_2 _score_2 _cellnumber_2) (break `/Game/Blueprints/S_PlayerData` (`|GetArrayItem` _playerlist)))
  (if (`KismetSystemLibrary.IsValid` (`self.PrevCard`))
    (bind _returnvalue (`self.TestPair` (`KismetMathLibrary.Conv_ByteToInt` (`/Game/Memory/Blueprint/BP_Card.Color` Card)) (`KismetMathLibrary.Conv_ByteToInt` (`/Game/Memory/Blueprint/BP_Card.Color` (`self.PrevCard`)))))
    (if _returnvalue
      (set `self.Score` (+ (`self.Score`) 10))
      (`self.UpdateScore` (`self.Score`))
      (`self.K2_DestroyActor` Card)
      (`self.K2_DestroyActor` (`self.PrevCard`))
      (else
        (`MemoryCard.TurnCard` Card)
        (`MemoryCard.TurnCard` (`self.PrevCard`))))
    (set `self.PrevCard` null)
    (if true
      (`|ExecutionSequence`
        (:`then_0`
          (bind _playercellnumber (`/Game/Blueprints/BP_GameInstance.GetPlayerCellNumberByPlayerId` (`self.GI_Ref`) 0))
          (if (== _playercellnumber 3)
            (`KismetArrayLibrary.Array_Set` _playerlist 0 (make `/Game/Blueprints/S_PlayerData` _playerid_2 (+ _score_2 (`self.MemoryScore`)) _cellnumber_2))
            (`GameplayStatics.OpenLevelBySoftObjectPtr` "/Game/Maps/Test_map.Test_map" :!label _label)))
        (:`then_1`
          (bind _playercellnumber_2 (`/Game/Blueprints/BP_GameInstance.GetPlayerCellNumberByPlayerId` (`self.GI_Ref`) 1))
          (if (== _playercellnumber_2 3)
            (`KismetArrayLibrary.Array_Set` _playerlist_2 1 (make `/Game/Blueprints/S_PlayerData` _playerid (+ _score (`self.MemoryScore`)) _cellnumber))
            (goto _label)))))
    (else
      (set `self.PrevCard` Card))))

(fn `UserConstructionScript`)